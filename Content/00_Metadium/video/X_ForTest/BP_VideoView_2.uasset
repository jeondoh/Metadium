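; BP_VideoView_2 is a video screen actor that streams a looping URL video onto a mesh, with sound.
; Construction calls SetVideoDataTable and creates a MediaTexture; SetMediaPlayer creates a player, opens AVideoUrl and binds texture, sound and a dynamic TV material.
; In cinema areas, a BP_MetaPlayer overlapping the box triggers this setup once.
; BeginPlay is empty, so the non-cinema setup and widget play/pause binding are disconnected.
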(event OnComponentBeginOverlap(BoxComponent)
  (params (OverlappedComponent :type Primitive%20Component%20Object%20Reference) (OtherActor :type Actor%20Object%20Reference) (OtherComp :type Primitive%20Component%20Object%20Reference) (OtherBodyIndex :type Integer) (bFromSweep :type Boolean) (SweepResult :type Hit%20Result%20Structure%20%28by%20ref%29))
  (if (Variables|Default|GetIsCinemaArea)
    (bind _asbp_meta_player (Utilities|Casting|CastToBP_MetaPlayer OtherActor))
    (Utilities|IsValid _asbp_meta_player
      (:Is%20Valid
        (Utilities|FlowControl|DoOnce false
          (:Completed
            (CallFunction|SetMediaPlayer)))))))

(event Custom|WidgetOnPressed
  (bind _mediaplayer (Variables|Default|GetMediaPlayer))
  (if (Audio|Components|Audio|IsPlaying _mediaplayer)
    (Sequencer|Player|Pause _mediaplayer)
    (else
      (Media|MediaPlayer|Play _mediaplayer :!class /Script/MediaAssets.MediaPlayer))))

(event EventBeginPlay)

(fn ConstructionScript
  (Class|VideoViewActor|SetVideoDataTable)
  (bind _returnvalue (Game|ConstructObjectfromClass "/Script/MediaAssets.MediaTexture" self))
  (Variables|Default|SetMediaTexture _returnvalue))

(fn SetMediaPlayer
  (bind _returnvalue (Game|ConstructObjectfromClass "/Script/MediaAssets.MediaPlayer" self))
  (bind _output_get (Variables|Default|SetMediaPlayer _returnvalue))
  (Media|MediaSoundComponent|SetMediaPlayer (Variables|Default|GetMediaTexture) _output_get)
  (Class|MediaPlayer|OpenUrl (Variables|Default|GetMediaPlayer) (Utilities|String|ToString(Text) (Variables|Default|GetAVideoUrl)))
  (Media|MediaSoundComponent|SetMediaPlayer (Variables|Default|GetMediaSound) (Variables|Default|GetMediaPlayer))
  (bind _returnvalue_2 (Rendering|Material|CreateDynamicMaterialInstance (Variables|Default|GetStaticMeshComponent) 0 "/Game/00_Metadium/video/Mat/M_TV_Inst.M_TV_Inst" "None" :!class /Script/Engine.PrimitiveComponent))
  (Rendering|Material|SetTextureParameterValue _returnvalue_2 "MediaTexture" (Variables|Default|GetMediaTexture))
  (Components|Timeline|SetLooping (Variables|Default|GetMediaPlayer) true))