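; Video theater actor that streams three looping concert videos onto three material slots of one mesh, with sound from the first.
; When a BP_MetaPlayer first overlaps its box in a cinema area, SetMediaPlayer creates the players after a short delay, feeding media textures built at construction.
; Tick pauses and rewinds each stream as it starts, then restarts all three together after the first one's delay, lining up playback.
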(event OnComponentBeginOverlap(BoxComponent)
  (params (OverlappedComponent :type Primitive%20Component%20Object%20Reference) (OtherActor :type Actor%20Object%20Reference) (OtherComp :type Primitive%20Component%20Object%20Reference) (OtherBodyIndex :type Integer) (bFromSweep :type Boolean) (SweepResult :type Hit%20Result%20Structure%20%28by%20ref%29))
  (if (Variables|Default|GetIsCinemaArea)
    (bind _asbp_meta_player (Utilities|Casting|CastToBP_MetaPlayer OtherActor))
    (Utilities|IsValid _asbp_meta_player
      (:Is%20Valid
        (Utilities|FlowControl|DoOnce false
          (:Completed
            (Utilities|FlowControl|Delay 2.5)
            (Variables|Default|SetIsPlay true)
            (CallFunction|SetMediaPlayer)))))))

(event EventTick
  (params (DeltaSeconds :type Float%20%28single-precision%29))
  (bind _mediaplayer (Variables|Default|GetMediaPlayer))
  (bind _mediaplayer2 (Variables|Default|GetMediaPlayer2))
  (bind _mediaplayer3 (Variables|Default|GetMediaPlayer3))
  (if (Variables|Default|GetIsPlay)
    (if (not (Math|Boolean|ANDBoolean (Variables|Default|GetIsPause) (Variables|Default|GetIsPause2) (Variables|Default|GetIsPause3)))
      (Utilities|FlowControl|Sequence
        (:then_0
          (if (Audio|Components|Audio|IsPlaying _mediaplayer)
            (bind _returnvalue (Sequencer|Player|Pause _mediaplayer))
            (if _returnvalue
              (Class|MediaPlayer|Rewind (Variables|Default|GetMediaPlayer))
              (Variables|Default|SetIsPause true)
              (Utilities|FlowControl|Delay 2.0)
              (Media|MediaPlayer|Play (Variables|Default|GetMediaPlayer) :!class /Script/MediaAssets.MediaPlayer)
              (Media|MediaPlayer|Play (Variables|Default|GetMediaPlayer2) :!class /Script/MediaAssets.MediaPlayer)
              (Media|MediaPlayer|Play (Variables|Default|GetMediaPlayer3) :!class /Script/MediaAssets.MediaPlayer))))
        (:then_1
          (if (Audio|Components|Audio|IsPlaying _mediaplayer2)
            (bind _returnvalue_2 (Sequencer|Player|Pause _mediaplayer2))
            (if _returnvalue_2
              (Class|MediaPlayer|Rewind (Variables|Default|GetMediaPlayer2))
              (Variables|Default|SetIsPause2 true))))
        (:then_2
          (if (Audio|Components|Audio|IsPlaying _mediaplayer3)
            (bind _returnvalue_3 (Sequencer|Player|Pause _mediaplayer3))
            (if _returnvalue_3
              (Class|MediaPlayer|Rewind (Variables|Default|GetMediaPlayer3))
              (Variables|Default|SetIsPause3 true))))))))

(fn ConstructionScript
  (Class|VideoViewActor|SetVideoDataTable)
  (Utilities|FlowControl|Sequence
    (:then_0
      (bind _returnvalue (Game|ConstructObjectfromClass "/Script/MediaAssets.MediaTexture" self))
      (Variables|Default|SetMediaTexture _returnvalue))
    (:then_1
      (bind _returnvalue_2 (Game|ConstructObjectfromClass "/Script/MediaAssets.MediaTexture" self))
      (Variables|Default|SetMediaTexture2 _returnvalue_2))
    (:then_2
      (bind _returnvalue_3 (Game|ConstructObjectfromClass "/Script/MediaAssets.MediaTexture" self))
      (Variables|Default|SetMediaTexture3 _returnvalue_3))))

(fn SetMediaPlayer
  (Utilities|FlowControl|Sequence
    (:then_0
      (bind _returnvalue (Game|ConstructObjectfromClass "/Script/MediaAssets.MediaPlayer" self))
      (bind _output_get (Variables|Default|SetMediaPlayer _returnvalue))
      (Media|MediaSoundComponent|SetMediaPlayer (Variables|Default|GetMediaTexture) _output_get)
      (Class|MediaPlayer|OpenUrl (Variables|Default|GetMediaPlayer) "http://175.198.95.114:8000/static/IU_Concert.mp4")
      (Media|MediaSoundComponent|SetMediaPlayer (Variables|Default|GetMediaSound) (Variables|Default|GetMediaPlayer))
      (bind _returnvalue_2 (Rendering|Material|CreateDynamicMaterialInstance (Variables|Default|GetStaticMeshComponent) 0 "/Game/00_Metadium/video/Mat/M_TV_Consert_Inst.M_TV_Consert_Inst" "None" :!class /Script/Engine.PrimitiveComponent))
      (Rendering|Material|SetTextureParameterValue _returnvalue_2 "MediaTexture" (Variables|Default|GetMediaTexture))
      (Components|Timeline|SetLooping (Variables|Default|GetMediaPlayer) true))
    (:then_1
      (bind _returnvalue_3 (Game|ConstructObjectfromClass "/Script/MediaAssets.MediaPlayer" self))
      (bind _output_get_2 (Variables|Default|SetMediaPlayer2 _returnvalue_3))
      (Media|MediaSoundComponent|SetMediaPlayer (Variables|Default|GetMediaTexture2) _output_get_2)
      (Class|MediaPlayer|OpenUrl (Variables|Default|GetMediaPlayer2) "http://175.198.95.114:8000/static/IU_Concert_02.mp4")
      (bind _returnvalue_4 (Rendering|Material|CreateDynamicMaterialInstance (Variables|Default|GetStaticMeshComponent) 1 "/Game/00_Metadium/video/Mat/M_TV_Consert_Inst.M_TV_Consert_Inst" "None" :!class /Script/Engine.PrimitiveComponent))
      (Rendering|Material|SetTextureParameterValue _returnvalue_4 "MediaTexture" (Variables|Default|GetMediaTexture2))
      (Components|Timeline|SetLooping (Variables|Default|GetMediaPlayer2) true))
    (:then_2
      (bind _returnvalue_5 (Game|ConstructObjectfromClass "/Script/MediaAssets.MediaPlayer" self))
      (bind _output_get_3 (Variables|Default|SetMediaPlayer3 _returnvalue_5))
      (Media|MediaSoundComponent|SetMediaPlayer (Variables|Default|GetMediaTexture3) _output_get_3)
      (Class|MediaPlayer|OpenUrl (Variables|Default|GetMediaPlayer3) "http://175.198.95.114:8000/static/IU_Concert_03.mp4")
      (bind _returnvalue_6 (Rendering|Material|CreateDynamicMaterialInstance (Variables|Default|GetStaticMeshComponent) 2 "/Game/00_Metadium/video/Mat/M_TV_Consert_Inst.M_TV_Consert_Inst" "None" :!class /Script/Engine.PrimitiveComponent))
      (Rendering|Material|SetTextureParameterValue _returnvalue_6 "MediaTexture" (Variables|Default|GetMediaTexture3))
      (Components|Timeline|SetLooping (Variables|Default|GetMediaPlayer3) true))))