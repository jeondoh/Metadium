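; BP_LightStick is a light stick actor that a motion controller can pick up, with a toggleable menu button.
; Pickup disables mesh physics, attaches the root to the controller's component, then sets the mesh's relative transform.
; Left and right LightStickMenu inputs share one FlipFlop that shows or hides MenuButton.
; Drop is empty, with its physics and detach nodes disconnected, so the stick stays attached.
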(event EventBeginPlay)

(event Collision|EventActorBeginOverlap
  (params (OtherActor :type Actor%20Object%20Reference)))

(event EventTick
  (params (DeltaSeconds :type Float%20%28single-precision%29)))

(event EventPickup
  (params (AttachTo :type Scene%20Component%20Object%20Reference))
  (Physics|SetSimulatePhysics (Variables|Debug|GetStaticMeshComponent) false)
  (Transformation|AttachComponentToComponent (VehicleSound|GetRootComponent) AttachTo "None" "KeepWorld" "KeepWorld" "KeepWorld" false)
  (Transformation|SetRelativeTransform (Variables|Debug|GetStaticMeshComponent) (Math|Transform|MakeTransform "0, 0, 0" "0, 0, 0" "1,1,1") false false))

(event EventDrop)

(event Input|ActionEvents|InputActionLightStickMenuL
  (params (Key :type Key%20Structure))
  (:Pressed
    (Utilities|FlowControl|FlipFlop
      (:A
        (Rendering|SetVisibility (Variables|Default|GetMenuButton) true false))
      (:B
        (Rendering|SetVisibility (Variables|Default|GetMenuButton) false false)))))

(event Input|ActionEvents|InputActionLightStickMenuR
  (params (Key :type Key%20Structure))
  (:Pressed
    (Utilities|FlowControl|FlipFlop
      (:A
        (Rendering|SetVisibility (Variables|Default|GetMenuButton) true false))
      (:B
        (Rendering|SetVisibility (Variables|Default|GetMenuButton) false false)))))

(fn ConstructionScript)