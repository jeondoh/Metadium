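; VR button actor, BP_LightStickButton, that switches BP_MetaPlayer into camera mode or map mode.
; Each mode triggers from a box overlap or a W_CheckPressed widget press bound on BeginPlay.
; The switch sets the mode flag, hides the menu and loads the camera screen or minimap widget, with camera mode also calling OutView.
; Physical presses use helpers that rumble the motion controller and animate the button down and back up, guarded by IsPressed.
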(event OnComponentBeginOverlap(CameraButtonBox)
  (params (OverlappedComponent :type Primitive%20Component%20Object%20Reference) (OtherActor :type Actor%20Object%20Reference) (OtherComp :type Primitive%20Component%20Object%20Reference) (OtherBodyIndex :type Integer) (bFromSweep :type Boolean) (SweepResult :type Hit%20Result%20Structure%20%28by%20ref%29))
  ;[0.2235 1 0.4] 카메라모드 버튼과 물리적 반응
  (|누르면내려가 OtherActor)
  (CallFunction|InverttoCameraMode)
  (|누르고나서올라가))

(event OnComponentBeginOverlap(MapButtonBox)
  (params (OverlappedComponent :type Primitive%20Component%20Object%20Reference) (OtherActor :type Actor%20Object%20Reference) (OtherComp :type Primitive%20Component%20Object%20Reference) (OtherBodyIndex :type Integer) (bFromSweep :type Boolean) (SweepResult :type Hit%20Result%20Structure%20%28by%20ref%29))
  ;[0.5176 0.8588 1] 맵모드 버튼과 물리적 반응
  (|누르면내려가 OtherActor)
  (CallFunction|InverttoMapMode)
  (|누르고나서올라가))

(event Custom|InvertToCameraMode
  ;[0.2235 1 0.4] 카메라모드 진입
  ;;[0 0 0] 3인칭 시점
  (bind _asbp_meta_player (Utilities|Casting|CastToBP_MetaPlayer (Game|Player|GetPlayerPawn 0)))
  (Default|OutView _asbp_meta_player)
  (Variables|/Game/00_Metadium/Player/BP_MetaPlayer.BP_MetaPlayer_C|SetCameraMode _asbp_meta_player true)
  (Default|UnSeenMenuWidget _asbp_meta_player)
  ;;[0 0 0] 카메라전용UI
  (bind _returnvalue (UserInterface|CreateWidget "/Game/00_Metadium/Player/W_CameraModeScreen.W_CameraModeScreen_C"))
  (UserInterface|SetWidget (Variables|/Game/00_Metadium/Player/BP_MetaPlayer.BP_MetaPlayer_C|GetWidget _asbp_meta_player) _returnvalue))

(event Custom|VRinteractionCamerabutton
  ;[0.2235 1 0.4] 카메라모드 버튼과 VR상호작용
  (CallFunction|InverttoCameraMode))

(event Custom|InvertToMapMode
  ;[0.5176 0.8588 1] 코멘트
  ;;[0 0 0] 맵전용 UI
  (bind _asbp_meta_player (Utilities|Casting|CastToBP_MetaPlayer (Game|Player|GetPlayerPawn 0)))
  (bind _returnvalue (UserInterface|CreateWidget "/Game/00_Metadium/Player/W_MiniMap.W_MiniMap_C"))
  (UserInterface|SetWidget (Variables|/Game/00_Metadium/Player/BP_MetaPlayer.BP_MetaPlayer_C|GetWidget1 _asbp_meta_player) _returnvalue)
  (Variables|/Game/00_Metadium/Player/BP_MetaPlayer.BP_MetaPlayer_C|SetMapMode _asbp_meta_player true)
  (Default|UnSeenMenuWidget _asbp_meta_player))

(event Custom|VRinteractionMapbutton
  ;[0.5176 0.8588 1] 맵모드 버튼과 VR상호작용
  (CallFunction|InverttoMapMode))

(event EventBeginPlay
  (Utilities|FlowControl|Sequence
    (:then_0
      ;[0.2235 1 0.4] 카메라모드 버튼과 VR상호작용
      (bind _asw_check_pressed (Utilities|Casting|CastToW_CheckPressed (UserInterface|GetWidget (Variables|Default|GetWidgetForCamera))))
      (EventDispatchers|BindEventtoOnPressed (Variables|/Game/00_Metadium/Player/IUbongButton/W_CheckPressed.W_CheckPressed_C|GetPressCheckButton _asw_check_pressed) (delegate Custom|VRinteractionCamerabutton)))
    (:then_1
      ;[0.5176 0.8588 1] 맵모드 버튼과 VR상호작용
      (bind _asw_check_pressed_2 (Utilities|Casting|CastToW_CheckPressed (UserInterface|GetWidget (Variables|Default|GetWidgetForMap))))
      (EventDispatchers|BindEventtoOnPressed (Variables|/Game/00_Metadium/Player/IUbongButton/W_CheckPressed.W_CheckPressed_C|GetPressCheckButton _asw_check_pressed_2) (delegate Custom|VRinteractionMapbutton)))))

(event Collision|EventActorBeginOverlap
  (params (OtherActor :type Actor%20Object%20Reference)))

(event EventTick
  (params (DeltaSeconds :type Float%20%28single-precision%29)))

(fn ConstructionScript)