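; IU light stick (IUbong) actor whose logo and inner plane glow in changeable colors.
; Construction creates dynamic materials for the stick's parts, keeping the logo and inner-plane instances for color changes, and detaches LightStickMenu.
; Eight ChangeColor events apply preset color pairs, while on Custom_Map BeginPlay loops ColorRandomChange every five seconds.
; AttachBong re-parents LightStickMenu to the root at a fixed relative transform, and DetachBong releases it.
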(event Custom|DetachBong
  (Transformation|DetachFromComponent (Variables|Default|GetLightStickMenu) "KeepRelative" "KeepRelative" "KeepRelative" true))

(event Custom|ChangeColor8
  ;[0.882 0.4202 1] ChangingColor
  (Rendering|Material|SetVectorParameterValue (Variables|Default|GetDynamicMaterialLogo) "Light" "(R=0.000000,G=0.029218,B=0.984375,A=1.000000)" :!class /Script/Engine.MaterialInstanceDynamic)
  (Rendering|Material|SetVectorParameterValue (Variables|Default|GetDynamicMaterialInnerPlane) "Light" "(R=0.423786,G=0.006914,B=1.000000,A=1.000000)" :!class /Script/Engine.MaterialInstanceDynamic))

(event Custom|ChangeColor5
  ;[0.882 0.4202 1] ChangingColor
  (Rendering|Material|SetVectorParameterValue (Variables|Default|GetDynamicMaterialLogo) "Light" "(R=0.106782,G=0.109123,B=0.984375,A=1.000000)" :!class /Script/Engine.MaterialInstanceDynamic)
  (Rendering|Material|SetVectorParameterValue (Variables|Default|GetDynamicMaterialInnerPlane) "Light" "(R=0.151058,G=0.910293,B=1.000000,A=1.000000)" :!class /Script/Engine.MaterialInstanceDynamic))

(event Custom|ChangeColor6
  ;[0.882 0.4202 1] ChangingColor
  (Rendering|Material|SetVectorParameterValue (Variables|Default|GetDynamicMaterialLogo) "Light" "(R=0.984375,G=0.237404,B=0.000000,A=1.000000)" :!class /Script/Engine.MaterialInstanceDynamic)
  (Rendering|Material|SetVectorParameterValue (Variables|Default|GetDynamicMaterialInnerPlane) "Light" "(R=1.000000,G=0.789384,B=0.101264,A=1.000000)" :!class /Script/Engine.MaterialInstanceDynamic))

(event Custom|ChangeColor7
  ;[0.882 0.4202 1] ChangingColor
  (Rendering|Material|SetVectorParameterValue (Variables|Default|GetDynamicMaterialLogo) "Light" "(R=0.583951,G=0.028510,B=1.000000,A=1.000000)" :!class /Script/Engine.MaterialInstanceDynamic)
  (Rendering|Material|SetVectorParameterValue (Variables|Default|GetDynamicMaterialInnerPlane) "Light" "(R=0.942028,G=0.142790,B=1.000000,A=1.000000)" :!class /Script/Engine.MaterialInstanceDynamic))

(event Custom|AttachBong
  (Transformation|AttachComponentToComponent (Variables|Default|GetLightStickMenu) (Variables|Default|GetDefaultSceneRoot) "None" "KeepRelative" "KeepRelative" "KeepRelative" true)
  (Transformation|SetRelativeTransform (Variables|Default|GetLightStickMenu) (Math|Transform|MakeTransform "-0.505071,-0.430458,14.910926" "70.000000,180.000000,0.000000" "0.200000,0.200000,0.200000") false false))

(event Custom|ChangeColor1
  ;[0.882 0.4202 1] ChangingColor
  (Rendering|Material|SetVectorParameterValue (Variables|Default|GetDynamicMaterialLogo) "Light" "(R=0.606299,G=0.110624,B=0.984375,A=1.000000)" :!class /Script/Engine.MaterialInstanceDynamic)
  (Rendering|Material|SetVectorParameterValue (Variables|Default|GetDynamicMaterialInnerPlane) "Light" "(R=1.000000,G=0.204164,B=0.906889,A=1.000000)" :!class /Script/Engine.MaterialInstanceDynamic))

(event Custom|ChangeColor2
  ;[0.882 0.4202 1] ChangingColor
  (Rendering|Material|SetVectorParameterValue (Variables|Default|GetDynamicMaterialLogo) "Light" "(R=0.984375,G=0.093464,B=0.271002,A=1.000000)" :!class /Script/Engine.MaterialInstanceDynamic)
  (Rendering|Material|SetVectorParameterValue (Variables|Default|GetDynamicMaterialInnerPlane) "Light" "(R=0.658281,G=0.217016,B=1.000000,A=1.000000)" :!class /Script/Engine.MaterialInstanceDynamic))

(event Custom|ChangeColor3
  ;[0.882 0.4202 1] ChangingColor
  (Rendering|Material|SetVectorParameterValue (Variables|Default|GetDynamicMaterialLogo) "Light" "(R=0.984375,G=0.026856,B=0.717296,A=1.000000)" :!class /Script/Engine.MaterialInstanceDynamic)
  (Rendering|Material|SetVectorParameterValue (Variables|Default|GetDynamicMaterialInnerPlane) "Light" "(R=1.000000,G=0.319799,B=0.886290,A=1.000000)" :!class /Script/Engine.MaterialInstanceDynamic))

(event Custom|ChangeColor4
  ;[0.882 0.4202 1] ChangingColor
  (Rendering|Material|SetVectorParameterValue (Variables|Default|GetDynamicMaterialLogo) "Light" "(R=0.000000,G=1.000000,B=0.235294,A=1.000000)" :!class /Script/Engine.MaterialInstanceDynamic)
  (Rendering|Material|SetVectorParameterValue (Variables|Default|GetDynamicMaterialInnerPlane) "Light" "(R=0.936054,G=1.000000,B=0.193868,A=1.000000)" :!class /Script/Engine.MaterialInstanceDynamic))

(event EventBeginPlay
  (bind _returnvalue (Game|GetCurrentLevelName true))
  (if (Utilities|Enum|Equal(Enum) _returnvalue "Custom_Map")
    (for _array_element (Variables|Default|GetLoop) :!label _label
      (Utilities|FlowControl|Delay 5.0)
      (CallFunction|ColorRandomChange)
      (if true
        (goto _label)))))

(fn ConstructionScript
  (bind _returnvalue (Rendering|Material|CreateDynamicMaterialInstance (Variables|Default|GetIUbong_MD_IUbong_Logo) 0 "/Game/00_Metadium/Player/IUbong/Material/M_IU_LightLogo_Inst.M_IU_LightLogo_Inst" "None" :!class /Script/Engine.PrimitiveComponent))
  (Variables|Default|SetDynamicMaterialLogo _returnvalue)
  (bind _returnvalue_2 (Rendering|Material|CreateDynamicMaterialInstance (Variables|Default|GetIUbong_MD_IUbong_Inner) 0 "/Game/00_Metadium/Player/IUbong/Material/M_IU_Inner_Light_Inst.M_IU_Inner_Light_Inst" "None" :!class /Script/Engine.PrimitiveComponent))
  (Variables|Default|SetDynamicMaterialInnerPlane _returnvalue_2)
  (Rendering|Material|CreateDynamicMaterialInstance (Variables|Default|GetIUbong_MD_IUbong_Stain) 0 "/Game/00_Metadium/Player/IUbong/Material/M_IU_Inside.M_IU_Inside" "None" :!class /Script/Engine.PrimitiveComponent)
  (Rendering|Material|CreateDynamicMaterialInstance (Variables|Default|GetIUbong_MD_IUbong_Glass1) 0 "/Game/00_Metadium/Player/IUbong/Material/M_Glass.M_Glass" "None" :!class /Script/Engine.PrimitiveComponent)
  (Rendering|Material|CreateDynamicMaterialInstance (Variables|Default|GetIUbong_MD_IUbong_Glass2) 0 "/Game/00_Metadium/Player/IUbong/Material/M_Glass.M_Glass" "None" :!class /Script/Engine.PrimitiveComponent)
  (Transformation|DetachFromComponent (Variables|Default|GetLightStickMenu) "KeepRelative" "KeepRelative" "KeepRelative" true))

(fn ColorRandomChange
  (Rendering|Material|SetVectorParameterValue (Variables|Default|GetDynamicMaterialLogo) "Light" (Math|Color|MakeColor (Math|Random|RandomFloatinRange 0.0 1.0) (Math|Random|RandomFloatinRange 0.0 1.0) (Math|Random|RandomFloatinRange 0.0 1.0)) :!class /Script/Engine.MaterialInstanceDynamic)
  (Rendering|Material|SetVectorParameterValue (Variables|Default|GetDynamicMaterialInnerPlane) "Light" (Math|Color|MakeColor (Math|Random|RandomFloatinRange 0.0 1.0) (Math|Random|RandomFloatinRange 0.0 1.0) (Math|Random|RandomFloatinRange 0.0 1.0)) :!class /Script/Engine.MaterialInstanceDynamic))