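; BP_ImageViewActor is an in-world actor that displays a web-loaded image with a titled caption.
; On BeginPlay it passes its URL to the BP_WGImageView widget to fetch the image, and fills the BP_Caption widget with its title and context text.
; While IsFocus is set, Tick turns the actor in yaw only to face the BP_MetaPlayer pawn.
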(event EventTick
  (params (DeltaSeconds :type Float%20%28single-precision%29))
  (if (Variables|Default|GetIsFocus)
    (bind _asbp_meta_player (Utilities|Casting|CastToBP_MetaPlayer (Game|Player|GetPlayerPawn 0)))
    (Transformation|SetActorRotation (Math|Rotator|MakeRotator 0.0 0.0 (.yaw (Math|Rotator|FindLookatRotation (Transformation|GetActorLocation) (Transformation|GetActorLocation _asbp_meta_player)))))))

(event EventBeginPlay
  (|CallParentFunction)
  (Utilities|FlowControl|Sequence
    (:then_0
      (bind _asbp_wgimage_view (Utilities|Casting|CastToBP_WGImageView (UserInterface|GetWidget (Variables|Default|GetWidgetComponent))))
      (Variables|/Script/Metadium.WebImageView|SetSourceImage (Variables|/Game/00_Metadium/image/BP_WGImageView.BP_WGImageView_C|GetBP_WebImageView_C_0 _asbp_wgimage_view) (Utilities|String|ToString(Text) (Variables|Default|GetAImageUrl)))
      (Class|WebImageView|SetImagefromWeb (Variables|/Game/00_Metadium/image/BP_WGImageView.BP_WGImageView_C|GetBP_WebImageView_C_0 _asbp_wgimage_view)))
    (:then_1
      (bind _asbp_caption (Utilities|Casting|CastToBP_Caption (UserInterface|GetWidget (Variables|Default|GetWidgetCaption))))
      (Variables|/Game/00_Metadium/HUD/BP_Caption.BP_Caption_C|SetCaptionText _asbp_caption (Utilities|String|ToString(Text) (Variables|Default|GetAImageContext)))
      (Variables|/Game/00_Metadium/HUD/BP_Caption.BP_Caption_C|SetCaptionTitleText _asbp_caption (Utilities|String|ToString(Text) (Variables|Default|GetAImageTitle))))))

(fn ConstructionScript)