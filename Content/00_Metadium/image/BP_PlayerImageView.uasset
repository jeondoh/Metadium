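; A grabbable actor that displays the local player's uploaded image on a widget component.
; On BeginPlay it appends BP_MetaPlayer's UploadFileName to a hard-coded HTTP server path, then has the BP_WGImageView widget load that URL from the web.
; Pickup from BP_MotionController turns off root physics and attaches the actor keeping world transform.
; Drop detaches it without re-enabling physics.
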(event EventBeginPlay
  (|CallParentFunction)
  (bind _asbp_wgimage_view (Utilities|Casting|CastToBP_WGImageView (UserInterface|GetWidget (Variables|Default|GetWidgetComponent))))
  (bind _output_get (Variables|/Script/Metadium.WebImageView|SetSourceImage (Variables|/Game/00_Metadium/image/BP_WGImageView.BP_WGImageView_C|GetBP_WebImageView_C_0 _asbp_wgimage_view) (Utilities|String|Append "http://175.198.95.114:8000/static/player/" (Variables|/Script/Metadium.MetaPlayer|GetUploadFileName (.AsBP%20Meta%20Player (Utilities|Casting|CastToBP_MetaPlayer (Game|Player|GetPlayerPawn 0)))))))
  (Variables|Default|SetAImageUrl (Utilities|Text|ToText(String) _output_get))
  (Class|WebImageView|SetImagefromWeb (Variables|/Game/00_Metadium/image/BP_WGImageView.BP_WGImageView_C|GetBP_WebImageView_C_0 _asbp_wgimage_view)))

(event EventPickup
  (params (AttachTo :type Scene%20Component%20Object%20Reference))
  (Physics|SetSimulatePhysics (Variables|Default|GetDefaultSceneRoot) false)
  (Transformation|AttachComponentToComponent (VehicleSound|GetRootComponent) AttachTo "None" "KeepWorld" "KeepWorld" "KeepWorld" false))

(event EventDrop
  (Transformation|DetachFromActor "KeepWorld" "KeepWorld" "KeepWorld"))

(fn ConstructionScript)